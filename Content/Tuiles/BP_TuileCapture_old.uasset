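; BP_TuileCapture_old is a map tile with a colour-coded state (Inactive, Discovered, Viable, Possessed) on which workers build houses.
; The construction script applies the state colour through UpdateTile.
; A worker entering trigger E is stopped and, after a five-second delay guarded by IsBuild, a BP_StabHouse spawns at the tile.
; The explorer overlap on Box is an unfinished stub with no effect.
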(event `self.Box.OnComponentBeginOverlap`
  (params (OverlappedComponent :type "PrimitiveComponent Object Reference") (OtherActor :type "Actor Object Reference") (OtherComp :type "PrimitiveComponent Object Reference") (OtherBodyIndex :type Integer) (bFromSweep :type Boolean) (SweepResult :type "HitResult Structure (by ref)"))
  (if (== OtherActor "/Game/Tuiles/BP_ExplorerUnit.BP_ExplorerUnit")
    (if (`self.IsDiscovered?`)
      _)))

(event `self.e.OnComponentBeginOverlap`
  (params (OverlappedComponent :type "PrimitiveComponent Object Reference") (OtherActor :type "Actor Object Reference") (OtherComp :type "PrimitiveComponent Object Reference") (OtherBodyIndex :type Integer) (bFromSweep :type Boolean) (SweepResult :type "HitResult Structure (by ref)"))
  (bind _asbp_worker_unit (cast `/Game/TopDown/Blueprints/PNJ/BP_WorkerUnit` OtherActor))
  (bind _output_get (set `self.As BP Worker Unit` _asbp_worker_unit))
  (if (not (`self.IsBuild?`))
    (`MovementComponent.StopMovementImmediately` (`Character.CharacterMovement` _output_get))
    (set `self.IsBuild?` true)
    (`KismetSystemLibrary.Delay` 5.0)
    (`|SpawnActorFromClass` "/Game/TopDown/Blueprints/Structures/BP_StabHouse.BP_StabHouse_C" (`self.GetTransform`) "AlwaysSpawn" "MultiplyWithRoot" null null)
    (set `self.IsBuild?` false)))

(fn `Update_Tile`
  (params (State :type "/Game/Tuiles/ENUM_TuileState Enum" :default "NewEnumerator0"))
  (bind _output_get (set `self.State` State))
  (`MeshComponent.SetColorParameterValueOnMaterials` (`self.TuileMesh`) "Color" (select `/Game/Tuiles/ENUM_TuileState` _output_get :`NewEnumerator0` (struct :`R` 0.192708 :`G` 0.192708 :`B` 0.192708 :`A` 1.0) :`NewEnumerator1` (struct :`R` 0.322917 :`G` 0.133671 :`B` 0.035376 :`A` 1.0) :`NewEnumerator2` (struct :`R` 0.612006 :`G` 0.791667 :`B` 0.181424 :`A` 1.0) :`NewEnumerator3` (struct :`G` 1.0 :`B` 0.078945 :`A` 1.0) :!type "LinearColor Structure")))

(fn `UserConstructionScript`
  (`self.Update_Tile` (`self.State`)))