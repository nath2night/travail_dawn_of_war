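; Capture tile that lets a worker unit build a BP_StabHouse on it.
; When a BP_WorkerUnit enters the E trigger, the tile halts its movement, waits a fixed delay, then spawns the house at its own transform.
; IsBuild blocks overlapping builds during the delay and clears afterwards, so later overlaps can build again.
; The Box explorer-discovery check and SecureBat are empty stubs.
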(event `self.Box.OnComponentBeginOverlap`
  (params (OverlappedComponent :type "PrimitiveComponent Object Reference") (OtherActor :type "Actor Object Reference") (OtherComp :type "PrimitiveComponent Object Reference") (OtherBodyIndex :type Integer) (bFromSweep :type Boolean) (SweepResult :type "HitResult Structure (by ref)"))
  (if (== OtherActor "/Game/Tuiles/BP_ExplorerUnit.BP_ExplorerUnit")
    (if (`self.IsDiscovered?`)
      _)))

(event `self.e.OnComponentBeginOverlap`
  (params (OverlappedComponent :type "PrimitiveComponent Object Reference") (OtherActor :type "Actor Object Reference") (OtherComp :type "PrimitiveComponent Object Reference") (OtherBodyIndex :type Integer) (bFromSweep :type Boolean) (SweepResult :type "HitResult Structure (by ref)"))
  (bind _asbp_worker_unit (cast `/Game/TopDown/Blueprints/PNJ/BP_WorkerUnit` OtherActor))
  (bind _output_get (set `self.As BP Worker Unit` _asbp_worker_unit))
  (if (not (`self.IsBuild?`))
    (`MovementComponent.StopMovementImmediately` (`Character.CharacterMovement` _output_get))
    (set `self.IsBuild?` true)
    (`KismetSystemLibrary.Delay` 5.0)
    (`|SpawnActorFromClass` "/Game/TopDown/Blueprints/Structures/BP_StabHouse.BP_StabHouse_C" (`self.GetTransform`) "AlwaysSpawn" "MultiplyWithRoot" null null)
    (set `self.IsBuild?` false)))

(fn `Secure_Bat`)

(fn `UserConstructionScript`)