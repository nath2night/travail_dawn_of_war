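; Base map tile that moves through Inactive, Discovered, Viable and Possessed states, recoloring its mesh via UpdateState.
; SetNextState advances the tile one state only if an overlapping neighbor in BoxNearTiles is Possessed.
; Box overlaps track the actor on the tile for a work-in-progress Discovering event, using a Timeline to progress explorer discovery.
; Discovering sets State directly, bypassing the color update, and has an empty branch plus debug prints.
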(event `SetNextState`
  (set `self.InContactWithPossessedTile` false)
  (for _array_element (`PrimitiveComponent.GetOverlappingActors` (`self.BoxNearTiles`) "BP_TuileParent_C")
    (bind _asbp_tuile_parent (cast `/Game/Tuiles/BP_TuileParent` _array_element))
    (if (`|EnumEquality` (`/Game/Tuiles/BP_TuileParent.State` _asbp_tuile_parent) "NewEnumerator3")
      (set `self.InContactWithPossessedTile` true)))
  (if (`self.InContactWithPossessedTile`)
    (`self.UpdateState` (select `/Game/Tuiles/ENUM_TuileState` (`self.State`) :`NewEnumerator0` "NewEnumerator1" :`NewEnumerator1` "NewEnumerator2" :`NewEnumerator2` "NewEnumerator3" :`NewEnumerator3` "NewEnumerator3" :!type "/Game/Tuiles/ENUM_TuileState Enum"))))

(event `self.ReceiveBeginPlay`
  (set `self.DiscoveringProgression` 0.0))

(event `self.Box.OnComponentBeginOverlap`
  (params (OverlappedComponent :type "PrimitiveComponent Object Reference") (OtherActor :type "Actor Object Reference") (OtherComp :type "PrimitiveComponent Object Reference") (OtherBodyIndex :type Integer) (bFromSweep :type Boolean) (SweepResult :type "HitResult Structure (by ref)"))
  (set `self.OverlapingActor` OtherActor)
  (set `self.IsOverlap?` true)
  (`KismetSystemLibrary.PrintString` "overlap"))

(event `Discovering`
  (`|ExecutionSequence`
    (:`then_0`
      (if (`self.IsOverlap?`)
        (if (`self.IsDiscovered?`)
          _
          (elif (== (`self.OverlapingActor`) "/Game/Tuiles/BP_ExplorerUnit.BP_ExplorerUnit")
            _))))
    (:`then_1`
      (while (and (`self.IsOverlap?`) (== (`self.OverlapingActor`) "/Game/Tuiles/BP_ExplorerUnit.BP_ExplorerUnit"))
        (bind (_direction _discoveringtrack) (`Timeline|Timeline` :!label _label)
          (:`Update`
            (bind _output_get (set `self.DiscoveringProgression` (`KismetMathLibrary.Lerp` 0.0 100.0 _discoveringtrack)))
            (`KismetSystemLibrary.PrintString` (`KismetStringLibrary.Conv_DoubleToString` _output_get)))))
      (if (== (`self.DiscoveringProgression`) 100.0)
        (set `self.State` "NewEnumerator1")
        (else
          (goto _label :!via `Stop`))))))

(event `self.Box.OnComponentEndOverlap`
  (params (OverlappedComponent :type "PrimitiveComponent Object Reference") (OtherActor :type "Actor Object Reference") (OtherComp :type "PrimitiveComponent Object Reference") (OtherBodyIndex :type Integer))
  (set `self.OverlapingActor` null)
  (set `self.IsOverlap?` false)
  (`KismetSystemLibrary.PrintString` "No overlap"))

(fn `GetNavigationState`
  (returns (State :type "/Game/Tuiles/ENUM_TuileState Enum"))
  (return (`self.State`)))

(fn `UpdateState`
  (params (State :type "/Game/Tuiles/ENUM_TuileState Enum" :default "NewEnumerator0"))
  (bind _output_get (set `self.State` State))
  (`MeshComponent.SetColorParameterValueOnMaterials` (`self.TuileMesh`) "Color" (select `/Game/Tuiles/ENUM_TuileState` _output_get :`NewEnumerator0` (struct :`R` 0.192708 :`G` 0.192708 :`B` 0.192708 :`A` 1.0) :`NewEnumerator1` (struct :`R` 0.322917 :`G` 0.133671 :`B` 0.035376 :`A` 1.0) :`NewEnumerator2` (struct :`R` 0.612006 :`G` 0.791667 :`B` 0.181424 :`A` 1.0) :`NewEnumerator3` (struct :`G` 1.0 :`B` 0.078945 :`A` 1.0) :!type "LinearColor Structure")))

(fn `UserConstructionScript`
  (`self.UpdateState` (`self.State`)))