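; BP_Tuile_Capture is a map tile that units discover or make viable by entering its Box trigger.
; A BP_ExplorerUnit overlap starts a timer that sets the tile to Discovered, cancelled if the explorer leaves early.
; A BP_Constructor overlap halts that worker and, after a delay, spawns a BP_StabHouse and sets the tile to Viable, without checking prior state.
; Each state change recolors TuileMesh through a material color parameter.
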(event `self.Box.OnComponentBeginOverlap`
  (params (OverlappedComponent :type "PrimitiveComponent Object Reference") (OtherActor :type "Actor Object Reference") (OtherComp :type "PrimitiveComponent Object Reference") (OtherBodyIndex :type Integer) (bFromSweep :type Boolean) (SweepResult :type "HitResult Structure (by ref)"))
  (`|ExecutionSequence`
    (:`then_0`
      (bind _asbp_constructor (cast `/Game/TopDown/Blueprints/PNJ/BP_Constructor` OtherActor))
      (bind _output_get (set `self.As BP NWorker` _asbp_constructor))
      (if (not (`self.IsBuild? `))
        (`MovementComponent.StopMovementImmediately` (`Character.CharacterMovement` _output_get))
        (set `self.IsBuild? ` true)
        (`KismetSystemLibrary.Delay` 5.0)
        (`|SpawnActorFromClass` "/Game/TopDown/Blueprints/Structures/BP_StabHouse.BP_StabHouse_C" (`self.GetTransform`) "AlwaysSpawn" "MultiplyWithRoot" null null)
        (set `self.IsBuild? ` false)
        (`self.Viabilisation`)))
    (:`then_1`
      (cast `/Game/Tuiles/BP_ExplorerUnit` OtherActor)
      (if (not (`self.IsInactive?`))
        (set `self.IsInactive?` true)
        (bind _returnvalue (`KismetSystemLibrary.K2_SetTimerDelegate` (delegate `Discoverin`) 6.0))))))

(event `Discoverin`
  (`self.Discover`))

(event `self.Box.OnComponentEndOverlap`
  (params (OverlappedComponent :type "PrimitiveComponent Object Reference") (OtherActor :type "Actor Object Reference") (OtherComp :type "PrimitiveComponent Object Reference") (OtherBodyIndex :type Integer))
  (cast `/Game/Tuiles/BP_ExplorerUnit` OtherActor)
  (set `self.IsInactive?` false)
  (`KismetSystemLibrary.K2_ClearAndInvalidateTimerHandle` (stale `self.Box.OnComponentBeginOverlap` _returnvalue)))

(fn `Discover`
  (bind _output_get (set `self.State` "NewEnumerator1"))
  (`MeshComponent.SetColorParameterValueOnMaterials` (`self.TuileMesh`) "Color" (select `/Game/Tuiles/ENUM_TuileState` _output_get :`NewEnumerator0` (struct :`R` 0.192708 :`G` 0.192708 :`B` 0.192708 :`A` 1.0) :`NewEnumerator1` (struct :`R` 0.322917 :`G` 0.133671 :`B` 0.035376 :`A` 1.0) :`NewEnumerator2` (struct :`R` 0.612006 :`G` 0.791667 :`B` 0.181424 :`A` 1.0) :`NewEnumerator3` (struct :`G` 1.0 :`B` 0.078945 :`A` 1.0) :!type "LinearColor Structure")))

(fn `UserConstructionScript`
  (`parent.UserConstructionScript`))

(fn `Viabilisation`
  (bind _output_get (set `self.State` "NewEnumerator2"))
  (`MeshComponent.SetColorParameterValueOnMaterials` (`self.TuileMesh`) "Color" (select `/Game/Tuiles/ENUM_TuileState` _output_get :`NewEnumerator0` (struct :`R` 0.192708 :`G` 0.192708 :`B` 0.192708 :`A` 1.0) :`NewEnumerator1` (struct :`R` 0.322917 :`G` 0.133671 :`B` 0.035376 :`A` 1.0) :`NewEnumerator2` (struct :`R` 0.612006 :`G` 0.791667 :`B` 0.181424 :`A` 1.0) :`NewEnumerator3` (struct :`G` 1.0 :`B` 0.078945 :`A` 1.0) :!type "LinearColor Structure")))